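; Enemy AI character that fights the player with melee combos and leaping attacks, driven by Blueprint logic.
; PawnSensing sets the target, and a looping timer alternates between approaching to attack and strafing while attack counts recharge.
; Tick faces the target and feeds strafe direction to the AnimInstance, while capsule hits box-trace to change blocked strafes.
; Interface messages carry sphere-overlap damage; incoming hits trigger directional reactions, knockback stun or death.
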(event `self.ReceiveBeginPlay`
  (`KismetSystemLibrary.Delay` 4.0)
  (`self.CombatStart`)
  (bind _asbp_player_enemy (cast `/Game/Blueprints/BP_PlayerEnemy` (`GameplayStatics.GetPlayerCharacter` 0) :!label _label)
    (:`then`
      (`/Engine/EditorBlueprintResources/StandardMacros.IsValid` _asbp_player_enemy))
    (:`CastFailed`
      (`KismetSystemLibrary.Delay` 0.2)
      (goto _label))))

(event `self.PawnSensing.OnSeePawn`
  (params (Pawn :type "Pawn Object Reference"))
  ;[0 0 0] On See Pawn
  (set `self.Target` Pawn)
  (`/Engine/EditorBlueprintResources/StandardMacros.DoOnce` false
    (:`Completed`
      (set `self.EnableTick` false)
      (`KismetSystemLibrary.Delay` 1.0) ; Just for initialization purpose
      (`self.RotateToPlayer`))))

(event `self.ReceiveTick`
  (params (DeltaSeconds :type "Float (single-precision)"))
  (bind (_returnvalue_roll _returnvalue_pitch _returnvalue_yaw) (`KismetMathLibrary.BreakRotator` (`KismetMathLibrary.NormalizedDeltaRotator` (`KismetMathLibrary.Conv_VectorToRotator` (`self.StrafeVector`)) (`self.GetControlRotation`))))
  ;[0 0 0] Strafe Logic
  (`self.GeneralCheck`
    (:`Can`
      (bind _target (`self.Target`)
        (:`then`
          (bind _alive_ (message `/Game/Blueprints/BPI_Combat.INT_isAlive?` _target))
          (if _alive_
            (if (`self.EnableTick`)
              (switch `/Game/Blueprints/E_MoveDirection` (`self.AIMovementDirection`)
                (:`NewEnumerator0`
                  (set `self.StrafeVector` (0.0 0.0 0.0)))
                (:`NewEnumerator1`
                  (set `self.EnableTick` false))
                (:`NewEnumerator2`
                  (set `self.StrafeVector` (* (`self.GetActorForwardVector`) (`self.MinusOne`))))
                (:`NewEnumerator3`
                  (set `self.StrafeVector` (* (`self.GetActorRightVector`) (`self.MinusOne`))))
                (:`NewEnumerator4`
                  (set `self.StrafeVector` (`self.GetActorRightVector`))))
              (`self.AddMovementInput` (`self.StrafeVector`)) ; Prepare for directional movement
              (message `/Game/Blueprints/BPI_Combat.INT_DirectionValue` (`self.CastAnimIns`) (select `bool` (`self.DirectionalMove?`) :`true` _returnvalue_yaw))
              (bind _target_2 (`self.Target`)
                (:`then`
                  (bind (_returnvalue_roll_2 _returnvalue_pitch_2 _returnvalue_yaw_2) (`KismetMathLibrary.BreakRotator` (`KismetMathLibrary.FindLookAtRotation` (`self.K2_GetActorLocation`) (`self.K2_GetActorLocation` _target_2))))
                  (`self.K2_SetActorRotation` (`KismetMathLibrary.MakeRotator` 0.0 0.0 _returnvalue_yaw_2)))
                (:`else`)))
            (else
              (`AnimInstance.StopSlotAnimation` (`self.CastAnimIns`) 0.25 "DefaultSlot"))))
        (:`else`)))))

(event `CombatStart`
  ;[0 0 0] Combat Main Logic
  (bind _returnvalue (`KismetSystemLibrary.K2_SetTimerDelegate` (delegate `CombatLogic`) 0.2 true))
  (set `self.CombatStartHandle` _returnvalue))

(event `RotateToPlayer`
  ;[0 0 0] Rotate to player if relative angle is over 30 (absolute value)
)

(event `CombatLogic`
  ;[0 0 0] Combat Main Logic
  (bind _target (`self.Target`)
    (:`then`
      (bind _alive_ (message `/Game/Blueprints/BPI_Combat.INT_isAlive?` _target))
      (if (and _alive_ (not (`self.Dead`)) (`self.AllowBehave?`) (`self.EnableTick`))
        (if (<= (`self.AttackCounts`) 0)
          ;;[1 1 1] 1. Recharge Attack counts
          ;; 2. Start to strafe
          (`|ExecutionSequence`
            (:`then_0`
              (`KismetSystemLibrary.Delay` 5.0) ; Attack after delay
              (set `self.AttackCounts` (`KismetMathLibrary.RandomIntegerInRange` 2 3))
              (`self.NextAttack`))
            (:`then_1`
              (`/Engine/EditorBlueprintResources/StandardMacros.DoOnce` false :!label _label_2
                (:`Completed`
                  (set `self.Strafe` true :!label _label_3)
                  (if (and (<= (`self.TargetDistance`) 200.0) (not (`self.Blocking`)))
                    (set `self.AIMovementDirection` "NewEnumerator2")
                    (elif (`KismetMathLibrary.RandomBool`)
                      (set `self.AIMovementDirection` "NewEnumerator3")
                      (else
                        (set `self.AIMovementDirection` "NewEnumerator4"))))))))
          (else
            (`/Engine/EditorBlueprintResources/StandardMacros.DoOnce` false :!label _label_4
              (:`Completed`
                (`|ExecutionSequence`
                  (:`then_0`
                    (set `self.Strafe` false)
                    (set `self.AIMovementDirection` "NewEnumerator1")
                    (if (<= (`self.TargetDistance`) 800.0)
                      (set `self.AIAttackType` "NewEnumerator0")
                      (set `self.AttackDistance` 150.0)
                      (else
                        (set `self.AIAttackType` "NewEnumerator1")
                        (set `self.AttackDistance` 2000.0)))
                    (`self.MoveToTarget`))
                  (:`then_1`
                    (goto _label_2 :!via `Reset`)))))))))
    (:`else`)))

(event `NextAttack`
  ;[0 0 0] Combat Main Logic
  (goto _label_4 :!via `Reset`))

(event `self.CapsuleComponent.OnComponentHit`
  (params (HitComponent :type "PrimitiveComponent Object Reference") (OtherActor :type "Actor Object Reference") (OtherComp :type "PrimitiveComponent Object Reference") (NormalImpulse :type "Vector Structure") (Hit :type "HitResult Structure (by ref)"))
  ;[0 0 0] Collision Check
  (if (`self.Strafe`)
    (`/Engine/EditorBlueprintResources/StandardMacros.DoOnce` false :!label _label_5
      (:`Completed`
        (bind (_outhit _returnvalue) (`KismetSystemLibrary.BoxTraceSingleForObjects` (`self.K2_GetActorLocation`) (select `byte` (`self.AIMovementDirection`) :`0` (0.0 0.0 0.0) :`1` (0.0 0.0 0.0) :`2` (+ (`self.K2_GetActorLocation`) (* (* (`self.GetActorForwardVector`) (`self.MinusOne`)) (`self.CollisionCheckDistance`))) :`3` (+ (`self.K2_GetActorLocation`) (* (* (`self.GetActorRightVector`) (`self.MinusOne`)) (`self.CollisionCheckDistance`))) :`4` (+ (`self.K2_GetActorLocation`) (* (`self.GetActorRightVector`) (`self.CollisionCheckDistance`)))) (50.0 50.0 50.0) (struct) (`|MakeArray` "ObjectTypeQuery1" "ObjectTypeQuery3" :!type "EObjectTypeQuery Enum")))
        (if _returnvalue
          (set `self.Blocking` true)
          (`self.StartStrafe`)
          (`KismetSystemLibrary.Delay` 0.2) ; Set re check interval
          (goto _label_5 :!via `Reset`))))))

(event `StartStrafe`
  ;[0 0 0] Combat Main Logic
  (goto _label_3))

(event `MoveToTarget`
  ;[0 0 0] Move to proper attack distance
  (`/Engine/EditorBlueprintResources/StandardMacros.DoOnce` false :!label _label_6
    (:`Completed`
      (set `self.StrafeVector` (0.0 0.0 0.0)) ; (0,0,0) means disable strafe vector
      (bind _target (`self.Target`)
        (:`then`
          (set `CharacterMovementComponent.MaxWalkSpeed` 800.0 (`self.CharacterMovement`))
          (`|AIMoveTo` self (0.0 0.0 0.0) _target (`self.AttackDistance`)
            (:`then`
              (set `self.DirectionalMove?` false))
            (:`OnSuccess`
              (set `self.AIMovementDirection` "NewEnumerator0")
              (set `self.DirectionalMove?` true)
              (set `CharacterMovementComponent.MaxWalkSpeed` 400.0 (`self.CharacterMovement`))
              (`self.StartAttacking`)
              (goto _label_6 :!via `Reset`))))
        (:`else`)))))

(event `StartAttacking`
  (bind _target (`self.Target`))
  ;[0 0 0] Attack combo
  (`self.GeneralCheck`
    (:`Can`
      (switch `/Game/Blueprints/E_AttackTypee` (`self.AIAttackType`)
        (:`NewEnumerator0`
          (`self.NormalAttack`
            (:`Completed`
              (`self.GeneralCheck` :!label _label_7
                (:`Can`
                  (if (<= (`self.TargetDistance`) 220.0)
                    (`self.StunAttack`
                      (:`Completed`
                        (`self.EndAttackCombo`)))
                    (else
                      (`self.EndAttackCombo`))))))))
        (:`NewEnumerator1`
          (bind _returnvalue (`self.PlayAnimMontage` null))
          (`|ExecutionSequence`
            (:`then_0`
              (`KismetSystemLibrary.Delay` (+ _returnvalue 0.2))
              (if (`KismetMathLibrary.RandomBoolWithWeight` 0.3)
                (goto _label_7)
                (else
                  (`self.EndAttackCombo`))))
            (:`then_1`
              (`/Engine/EditorBlueprintResources/StandardMacros.IsValid` _target
                (:`Is Valid`
                  (`KismetSystemLibrary.Delay` 0.3) ; Jump start time
                  (set `self.TargetPreLocation` (`self.K2_GetActorLocation` _target))
                  (bind (_direction _alpha) (`Timeline|JumpToTarget` :!via `PlayFromStart`)
                    (:`Update`
                      (`self.K2_SetActorLocation` (`KismetMathLibrary.VLerp` (`self.K2_GetActorLocation`) (+ (`self.TargetPreLocation`) (* (`self.GetActorForwardVector`) (`self.MinusOne`) (`self.JumpAttackLandDistance`))) _alpha)))))))))))))

(event `CustomEvent_1`
  (params (BaseDamage :type "Float (double-precision)") (Radius :type "Float (double-precision)") (SphereDistance :type "Float (double-precision)") (AdditionalInfo :type "Array of String (by ref)") (AdditionalInfoIndex :type Integer))
  ;[0 0 0] Cause Damage
  (`|ExecutionSequence`
    (:`then_0`
      (bind _outactors (`KismetSystemLibrary.SphereOverlapActors` (+ (`self.K2_GetActorLocation`) (* (`self.GetActorForwardVector`) SphereDistance)) Radius (`|MakeArray` "ObjectTypeQuery3" :!type "EObjectTypeQuery Enum") null (`|MakeArray` self :!type "Actor Object Reference")))
      (for _array_element _outactors
        (if (`self.ActorHasTag` _array_element "player")
          (message `/Game/Blueprints/BPI_Combat.INT_HitHandle` _outactors self BaseDamage AdditionalInfo AdditionalInfoIndex))))
    (:`then_1`)))

(event `CameraShake`
  ;[0 0 0] Attack combo
  (`PlayerCameraManager.StartCameraShake` :`self` (`GameplayStatics.GetPlayerCameraManager` 0)))

(event `QuickRotation`
  (bind (_returnvalue_roll _returnvalue_pitch _returnvalue_yaw) (`KismetMathLibrary.BreakRotator` (`self.K2_GetActorRotation`)))
  ;[0 0 0] Attack combo
  (bind (_direction _alpha) (`Timeline|ShortRotation` :!via `PlayFromStart` :!label _label_8)
    (:`Update`
      (bind _target (`self.Target`)
        (:`then`
          (bind (_returnvalue_roll_2 _returnvalue_pitch_2 _returnvalue_yaw_2) (`KismetMathLibrary.BreakRotator` (`KismetMathLibrary.FindLookAtRotation` (`self.K2_GetActorLocation`) (`self.K2_GetActorLocation` _target))))
          (bind (_returnvalue_roll_3 _returnvalue_pitch_3 _returnvalue_yaw_3) (`KismetMathLibrary.BreakRotator` (`KismetMathLibrary.RLerp` (`KismetMathLibrary.MakeRotator` 0.0 0.0 _returnvalue_yaw) (`KismetMathLibrary.MakeRotator` 0.0 0.0 _returnvalue_yaw_2) _alpha true)))
          (`self.K2_SetActorRotation` (`KismetMathLibrary.MakeRotator` 0.0 0.0 _returnvalue_yaw_3)))
        (:`else`
          (goto _label_8 :!via `Stop`))))))

(event `EndAttackCombo`
  ;[0 0 0] Attack combo
  (set `self.AttackCounts` (- (`self.AttackCounts`) 1))
  (`self.RotateToPlayer`))

(event `CustomEvent`
  (params (DamageCauser :type "Actor Object Reference") (FinalDamage :type "Float (double-precision)") (AdditionalInfo :type "Array of String (by ref)") (AdditionalInfoIndex :type Integer))
  ;[0 0 0] Hit Reaction
  (set `self.DamageCauser` DamageCauser)
  (if (not (`self.Dead`))
    (bind _output_get (set `self.CurHP` (`KismetMathLibrary.FClamp` (- (`self.CurHP`) FinalDamage) 0.0 (`self.MaxHP`))))
    (if (< _output_get 0.1)
      (`self.Death`)
      (elif (> (`KismetArrayLibrary.Array_Length` AdditionalInfo) 0)
        (if (== (`|GetArrayItem` AdditionalInfo AdditionalInfoIndex) "stun")
          (`self.Stun`)
          (else
            (if (`/Game/Blueprints/FLib_MCAI.FLib_FaceToFace?` DamageCauser self) :!label _label_9
              (`self.PlayAnimMontage` null) ; Lean backward
              (else
                (`self.PlayAnimMontage` null) ; Lean forward
              ))))
        (else
          (goto _label_9))))))

(event `Stun`
  ;[0 0 0] Hit Reaction
  (set `self.EnableTick` false) ; Do not rotate actively to player during stun
  (set `self.AllowBehave?` false) ; Disable movement logic temporily
  (`self.PlayAnimMontage` null)
  (`|ExecutionSequence`
    (:`then_0`
      (bind (_direction _alpha) (`Timeline|KnockBack` :!via `PlayFromStart`) ; KnockBack time 0.5s
        (:`Update`
          (bind _target (`self.Target`)
            (:`then`
              (`self.K2_SetActorLocation` (`KismetMathLibrary.VLerp` (`self.K2_GetActorLocation`) (+ (`self.K2_GetActorLocation`) (* (`self.GetActorForwardVector` _target) (`self.KnockBackDistance`))) _alpha)))
            (:`else`)))))
    (:`then_1`
      (`KismetSystemLibrary.Delay` 2.0) ; Stun duration
      (if (not (`self.Dead`))
        (`AnimInstance.Montage_Stop` (`self.CastAnimIns`) 0.0 null)
        (set `self.AllowBehave?` true)
        (set `self.EnableTick` true)
        (`self.NextAttack`)))))

(event `Death`
  ;[0 0 0] Death
  (set `self.Dead` true)
  (set `self.AllowBehave?` false))

(fn `INT_isAlive?`
  (returns (`Alive?` :type Boolean))
  (return false))

(fn `TurnInPlace`
  (params (R :type "Float (double-precision)"))
  (returns (RotationTime :type "Float (double-precision)") (NeedToRotate :type Boolean))
  (locals (L_RelativeRotation :type "Float (double-precision)") (L_RotationTime :type "Float (double-precision)" :default 0.0))
  (bind (_returnvalue_roll _returnvalue_pitch _returnvalue_yaw) (`KismetMathLibrary.BreakRotator` (`self.K2_GetActorRotation`)))
  (bind _l_relativerotation (`local.L_RelativeRotation`))
  (bind _l_relativerotation_2 (`local.L_RelativeRotation`))
  (bind _l_relativerotation_3 (`local.L_RelativeRotation`))
  (bind _l_relativerotation_4 (`local.L_RelativeRotation`))
  (bind _target (`self.Target`)
    (:`then`
      (bind (_returnvalue_roll_2 _returnvalue_pitch_2 _returnvalue_yaw_2) (`KismetMathLibrary.BreakRotator` (`KismetMathLibrary.FindLookAtRotation` (`self.K2_GetActorLocation`) (`self.K2_GetActorLocation` _target))))
      (set `local.L_RelativeRotation` (- _returnvalue_yaw_2 _returnvalue_yaw))
      (if (or (and (> _l_relativerotation_4 0.0) (<= _l_relativerotation_4 30.0)) (and (> _l_relativerotation_4 -360.0) (<= _l_relativerotation_4 -330.0)) (and (> _l_relativerotation_4 -30.0) (<= _l_relativerotation_4 0.0)) (and (> _l_relativerotation_4 330.0) (<= _l_relativerotation_4 360.0)))
        (return 0.0 false)
        (else
          (if (or (and (> _l_relativerotation_2 0.0) (<= _l_relativerotation_2 90.0)) (and (> _l_relativerotation_2 -360.0) (<= _l_relativerotation_2 -270.0)))
            (bind _returnvalue (`self.PlayAnimMontage` null))
            (set `local.L_RotationTime` _returnvalue)
            (elif (or (and (> _l_relativerotation_3 90.0) (<= _l_relativerotation_3 180.0)) (and (> _l_relativerotation_3 -270.0) (<= _l_relativerotation_3 -180.0)))
              (bind _returnvalue_2 (`self.PlayAnimMontage` null))
              (set `local.L_RotationTime` _returnvalue_2)
              (elif (or (and (> _l_relativerotation 180.0) (<= _l_relativerotation 270.0)) (and (> _l_relativerotation -180.0) (<= _l_relativerotation -90.0)))
                (bind _returnvalue_3 (`self.PlayAnimMontage` null))
                (set `local.L_RotationTime` _returnvalue_3)
                (else
                  (bind _returnvalue_4 (`self.PlayAnimMontage` null))
                  (set `local.L_RotationTime` _returnvalue_4)))))
          (return (`local.L_RotationTime`) true))))
    (:`else`)))

(fn `UserConstructionScript`)