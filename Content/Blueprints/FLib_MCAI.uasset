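; FLib_MCAI is a Blueprint function library with one check for whether SelfRef is facing a Target actor.
; It compares SelfRef's yaw with the look-at yaw from Target to SelfRef, returning true when the absolute difference is above 90 and up to 270 degrees.
; This puts Target in SelfRef's front half on the horizontal plane; despite the "FaceToFace" name, Target's rotation is ignored.
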(fn `FLib_FaceToFace?`
  (params (Target :type "Actor Object Reference") (SelfRef :type "Actor Object Reference"))
  (returns (`FaceToFace?` :type Boolean))
  (bind (_returnvalue_roll _returnvalue_pitch _returnvalue_yaw) (`KismetMathLibrary.BreakRotator` (`Actor.K2_GetActorRotation` SelfRef)))
  (bind (_returnvalue_roll_2 _returnvalue_pitch_2 _returnvalue_yaw_2) (`KismetMathLibrary.BreakRotator` (`KismetMathLibrary.FindLookAtRotation` (`Actor.K2_GetActorLocation` Target) (`Actor.K2_GetActorLocation` SelfRef))))
  (bind _returnvalue (`KismetMathLibrary.Abs` (- _returnvalue_yaw_2 _returnvalue_yaw)))
  (`/Engine/EditorBlueprintResources/StandardMacros.IsValid` Target
    (:`Is Valid`
      (`/Engine/EditorBlueprintResources/StandardMacros.IsValid` SelfRef
        (:`Is Valid`
          (return (and (> _returnvalue 90.0) (<= _returnvalue 270.0))))))))