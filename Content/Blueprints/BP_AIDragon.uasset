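; AI dragon enemy that fights the player with melee bites, ranged claw or ground-fire attacks, and a periodic flying fire-breath phase.
; PawnSensing sets the target, then a looping timer picks an attack by distance or fly cooldown, moves into range and runs montage combos.
; Timelines drive turning, takeoff, landing, fireballs and stun knockback.
; It also handles sphere-overlap damage, crosshair-widget HP display and ground or airborne death.
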(event `self.ReceiveBeginPlay`
  (`KismetSystemLibrary.Delay` 4.0)
  (`self.CombatStart`)
  (bind _asbp_player_pawn (cast `/Game/ThirdPersonCPP/Blueprints/BP_PlayerPawn` (`GameplayStatics.GetPlayerCharacter` 0) :!label _label)
    (:`then`
      (`/Engine/EditorBlueprintResources/StandardMacros.IsValid` _asbp_player_pawn))
    (:`CastFailed`
      (`KismetSystemLibrary.Delay` 0.2)
      (goto _label))))

(event `self.PawnSensing.OnSeePawn`
  (params (Pawn :type "Pawn Object Reference"))
  ;[0 0 0] On See Pawn
  (set `self.Target` Pawn)
  (`/Engine/EditorBlueprintResources/StandardMacros.DoOnce` false
    (:`Completed`
      (set `self.EnableTick` false)
      (`KismetSystemLibrary.Delay` 1.0) ; Just for initialization purpose
      (`self.RotateToPlayer`)
      (set `self.FlyCoolDown` 0)
      (`ActorComponent.Deactivate` (`self.PawnSensing`)))))

(event `self.ReceiveTick`
  (params (DeltaSeconds :type "Float (single-precision)"))
  (bind _foundwidgets (`WidgetBlueprintLibrary.GetAllWidgetsOfClass` "/Game/Blueprints/WBP_Crosshair.WBP_Crosshair_C"))
  (for _array_element _foundwidgets
    ;[0 0 0] Strafe Logic
    (`ProgressBar.SetPercent` (`/Game/Blueprints/WBP_Crosshair.ProgressBar_0` _array_element) (/ (`self.CurHP`) 60.0))
    (`self.GeneralCheck`
      (:`Can`
        (bind _target (`self.Target`)
          (:`then`
            (bind _alive_ (message `/Game/Blueprints/BPI_Combat.INT_isAlive?` _target))
            (if _alive_
              (if (`self.EnableTick`)
                (switch `/Game/Blueprints/E_MoveDirection` (`self.AIMovementDirection`)
                  (:`NewEnumerator0`
                    (set `self.StrafeVector` (0.0 0.0 0.0)))
                  (:`NewEnumerator1`
                    (set `self.EnableTick` false)))
                (bind _target_2 (`self.Target`)
                  (:`then`
                    (bind (_returnvalue_roll _returnvalue_pitch _returnvalue_yaw) (`KismetMathLibrary.BreakRotator` (`KismetMathLibrary.FindLookAtRotation` (`self.K2_GetActorLocation`) (`self.K2_GetActorLocation` _target_2))))
                    (`self.K2_SetActorRotation` (`KismetMathLibrary.MakeRotator` 0.0 0.0 _returnvalue_yaw)))
                  (:`else`)))
              (else
                (`AnimInstance.StopSlotAnimation` (`self.CastAnimIns`) 0.25 "DefaultSlot"))))
          (:`else`))))))

(event `CombatStart`
  ;[0 0 0] Combat Main Logic
  (bind _returnvalue (`KismetSystemLibrary.K2_SetTimerDelegate` (delegate `CombatLogic`) 0.2 true))
  (set `self.CombatStartHandle` _returnvalue))

(event `RotateToPlayer`
  (bind (_returnvalue_roll _returnvalue_pitch _returnvalue_yaw) (`KismetMathLibrary.BreakRotator` (`self.K2_GetActorRotation`)))
  ;[0 0 0] Rotate to player if relative angle is over 30 (absolute value)
  (`self.GeneralCheck`
    (:`Can`
      (`self.Target`
        (:`then`
          (bind (_rotationtime _needtorotate) (`self.TurnInPlace` 0.0))
          (if _needtorotate
            (`TimelineComponent.SetPlayRate` (`self.RotateCurve`) (/ 1.0 (select `bool` (`KismetMathLibrary.NearlyEqual_FloatFloat` _rotationtime) :`false` _rotationtime :`true` 1.0)))
            (bind (_direction _alpha) (`Timeline|RotateCurve` :!via `PlayFromStart` :!label _label_2)
              (:`Update`
                (bind _target (`self.Target`)
                  (:`then`
                    (bind (_returnvalue_roll_2 _returnvalue_pitch_2 _returnvalue_yaw_2) (`KismetMathLibrary.BreakRotator` (`KismetMathLibrary.FindLookAtRotation` (`self.K2_GetActorLocation`) (`self.K2_GetActorLocation` _target))))
                    (bind (_returnvalue_roll_3 _returnvalue_pitch_3 _returnvalue_yaw_3) (`KismetMathLibrary.BreakRotator` (`KismetMathLibrary.RLerp` (`KismetMathLibrary.MakeRotator` 0.0 0.0 _returnvalue_yaw) (`KismetMathLibrary.MakeRotator` 0.0 0.0 _returnvalue_yaw_2) _alpha true)))
                    (`self.K2_SetActorRotation` (`KismetMathLibrary.MakeRotator` 0.0 0.0 _returnvalue_yaw_3)))
                  (:`else`
                    (goto _label_2 :!via `Stop`))))
              (:`Finished`
                (`self.GeneralCheck` :!label _label_3
                  (:`Can`
                    (set `self.EnableTick` true) ; Make AI always face to player now
                    (`self.NextAttack`)))))
            (else
              (goto _label_3))))
        (:`else`)))))

(event `CombatLogic`
  ;[0 0 0] Combat Main Logic
  (bind _target (`self.Target`)
    (:`then`
      (bind _alive_ (message `/Game/Blueprints/BPI_Combat.INT_isAlive?` _target))
      (if (and _alive_ (not (`self.Dead`)) (`self.AllowBehave?`) (`self.EnableTick`))
        (if (<= (`self.AttackCounts`) 0)
          (`KismetSystemLibrary.Delay` 1.0) ; Attack after delay
          (set `self.AttackCounts` (`KismetMathLibrary.RandomIntegerInRange` 2 3))
          (`self.NextAttack`)
          (`/Engine/EditorBlueprintResources/StandardMacros.IncrementInt` (`self.FlyCoolDown`))
          (else
            (`/Engine/EditorBlueprintResources/StandardMacros.DoOnce` false :!label _label_4
              (:`Completed`
                (set `self.AIMovementDirection` "NewEnumerator1")
                (if (< (`self.FlyCoolDown`) 3)
                  (if (<= (`self.TargetDistance`) 900.0)
                    (set `self.AIAttackType` "NewEnumerator0")
                    (set `self.AttackDistance` 600.0)
                    (else
                      (set `self.AIAttackType` "NewEnumerator1")
                      (set `self.AttackDistance` 2400.0)))
                  (else
                    (set `self.FlyCoolDown` 0)
                    (set `self.AIAttackType` "NewEnumerator2")
                    (set `self.AttackDistance` 99999.0)))
                (`self.MoveToTarget`)))))))
    (:`else`)))

(event `NextAttack`
  ;[0 0 0] Combat Main Logic
  (goto _label_4 :!via `Reset`))

(event `MoveToTarget`
  ;[0 0 0] Move to proper attack distance
  (`/Engine/EditorBlueprintResources/StandardMacros.DoOnce` false :!label _label_5
    (:`Completed`
      (bind _target (`self.Target`)
        (:`then`
          (set `CharacterMovementComponent.MaxWalkSpeed` 1200.0 (`self.CharacterMovement`))
          (`|AIMoveTo` self (0.0 0.0 0.0) _target (`self.AttackDistance`) :!label _label_6
            (:`then`
              (set `self.DirectionalMove?` false))
            (:`OnSuccess`
              (set `self.AIMovementDirection` "NewEnumerator0")
              (set `self.DirectionalMove?` true)
              (set `CharacterMovementComponent.MaxWalkSpeed` 600.0 (`self.CharacterMovement`))
              (`self.StartAttacking`)
              (goto _label_5 :!via `Reset`))
            (:`OnFail`
              (`KismetSystemLibrary.Delay` 0.2)
              (goto _label_6))))
        (:`else`)))))

(event `StartAttacking`
  (bind _returnvalue (<= (`self.TargetDistance`) 600.0))
  ;[0 0 0] Attack combo
  (`self.GeneralCheck`
    (:`Can`
      (switch `/Game/Blueprints/E_AttackTypee` (`self.AIAttackType`)
        (:`NewEnumerator0`
          (if (not _returnvalue)
            (`self.BiteAttack`
              (:`Completed`
                _)))
          (`self.GeneralCheck`
            (:`Can`
              (if _returnvalue
                (`self.VeryNearAttack`
                  (:`Completed`
                    _)))
              (`self.EndAttackCombo`))))
        (:`NewEnumerator1`
          (if (`KismetMathLibrary.RandomBool`)
            (`self.ClawTwice`
              (:`Completed`
                _))
            (else
              (`self.SpitFireOnGround`
                (:`Completed`
                  _))))
          (`self.EndAttackCombo`))
        (:`NewEnumerator2`
          (`self.StartToFly`))))))

(event `FireStart`
  ;[1 1 1] Fire Damage
  (`ActorComponent.Activate` (`self.ParticleSystem`) false)
  (`SceneComponent.K2_SetWorldRotation` (`self.ParticleSystem`) (`KismetMathLibrary.FindLookAtRotation` (`SceneComponent.GetSocketLocation` (`self.Mesh`) "Socket_SpreadFire") (- (`self.K2_GetActorLocation` (`self.Target`)) (0.0 0.0 1500.0))) false false))

(event `CauseDamage`
  (params (BaseDamage :type "Float (double-precision)") (Radius :type "Float (double-precision)") (SphereDistance :type "Float (double-precision)") (AdditionalInfo :type "Array of String (by ref)") (AdditionalInfoIndex :type Integer))
  (bind _returnvalue (+ (`self.K2_GetActorLocation`) (* (`self.GetActorForwardVector`) SphereDistance)))
  ;[0 0 0] Cause Damage
  (set `self.AdditionalInfo` AdditionalInfo)
  (`|ExecutionSequence`
    (:`then_0`
      (bind _outactors (`KismetSystemLibrary.SphereOverlapActors` _returnvalue Radius (`|MakeArray` "ObjectTypeQuery3" :!type "EObjectTypeQuery Enum") null (`|MakeArray` self :!type "Actor Object Reference")))
      (for _array_element _outactors
        (if (`self.ActorHasTag` _array_element "player")
          (message `/Game/Blueprints/BPI_Combat.INT_HitHandle` _outactors self BaseDamage AdditionalInfo AdditionalInfoIndex))))
    (:`then_1`
      (`KismetSystemLibrary.DrawDebugSphere` _returnvalue Radius 12 (struct :`R` 0.034671 :`G` 1.0 :`A` 1.0) 5.0 6.0))))

(event `FireEnd`
  ;[1 1 1] Fire Damage
  (`ActorComponent.Deactivate` (`self.ParticleSystem`)))

(event `StartToFly`
  ;[0 0 0] Attack combo
  (bind _output_get (set `self.Fly?` true))
  (message `/Game/Blueprints/BPI_Combat.INT_SetFly` (`self.CastAnimIns`) _output_get)
  (`CharacterMovementComponent.SetMovementMode` (`self.CharacterMovement`) "MOVE_Flying" 0)
  (`self.QuickRotation`)
  (bind (_direction _alpha) (`Timeline|TakeOffCurve` :!via `PlayFromStart`)
    (:`Update`
      (`self.GeneralCheck`
        (:`Can`
          (`self.AddMovementInput` (0.0 0.0 1.0) _alpha))))
    (:`Finished`
      (`self.DuringFly`)
      (`self.QuickRotation`)
      (`KismetSystemLibrary.Delay` 0.3)
      (set `self.EnableTick` true))))

(event `self.ParticleSystem.OnParticleCollide`
  (params (EventName :type Name) (EmitterTime :type "Float (single-precision)") (ParticleTime :type Integer) (Location :type "Vector Structure") (Velocity :type "Vector Structure") (Direction :type "Vector Structure") (Normal :type "Vector Structure") (BoneName :type Name) (PhysMat :type "PhysicalMaterial Object Reference"))
  ;[1 1 1] Fire Damage
  (`KismetSystemLibrary.PrintString` "Hello")
  (bind _target (`self.Target`)
    (:`then`
      (if (== (`self.K2_GetActorLocation` _target) Location :`ErrorTolerance` (`self.DragonSpreadFireRange`))
        _
        (else
          _))
      (bind _asbp_player_pawn (cast `/Game/ThirdPersonCPP/Blueprints/BP_PlayerPawn` _target))
      (`/Game/ThirdPersonCPP/Blueprints/BP_PlayerPawn.DamagedByFire` _asbp_player_pawn))
    (:`else`)))

(event `DuringFly`
  ;[0 0 0] Attack combo
  (`self.GeneralCheck`
    (:`Can`
      (`self.PlayAnimMontage` "/Game/QuadrapedCreatures/MountainDragon/Animations/ANIM_MOUNTAIN_DRAGON_FlyStationarySpreadFire_Montage.ANIM_MOUNTAIN_DRAGON_FlyStationarySpreadFire_Montage" :!label _label_7)
      (`KismetSystemLibrary.Delay` 4.0)
      (if (< (`self.FIreCount`) 3)
        (set `self.FIreCount` (+ (`self.FIreCount`) 1))
        (goto _label_7)
        (else
          (set `self.FIreCount` 0)
          (`self.StartToLand`))))))

(event `StartToLand`
  ;[0 0 0] Attack combo
  (set `self.EnableTick` false)
  (bind (_direction _alpha) (`Timeline|타임라인_0` :!via `PlayFromStart`)
    (:`Update`
      (`self.GeneralCheck`
        (:`Can`
          (`self.AddMovementInput` (0.0 0.0 -1.0) _alpha))))
    (:`Finished`
      (bind _output_get (set `self.Fly?` false))
      (message `/Game/Blueprints/BPI_Combat.INT_SetFly` (`self.CastAnimIns`) _output_get)
      (`CharacterMovementComponent.SetMovementMode` (`self.CharacterMovement`) "MOVE_Walking" 0)
      (`self.EndAttackCombo`))))

(event `CameraShake`
  ;[0 0 0] Attack combo
  (`PlayerCameraManager.StartCameraShake` :`self` (`GameplayStatics.GetPlayerCameraManager` 0)))

(event `QuickRotation`
  (bind (_returnvalue_roll _returnvalue_pitch _returnvalue_yaw) (`KismetMathLibrary.BreakRotator` (`self.K2_GetActorRotation`)))
  ;[0 0 0] Attack combo
  (bind (_direction _alpha) (`Timeline|ShortRotation` :!via `PlayFromStart` :!label _label_8)
    (:`Update`
      (bind _target (`self.Target`)
        (:`then`
          (bind (_returnvalue_roll_2 _returnvalue_pitch_2 _returnvalue_yaw_2) (`KismetMathLibrary.BreakRotator` (`KismetMathLibrary.FindLookAtRotation` (`self.K2_GetActorLocation`) (`self.K2_GetActorLocation` _target))))
          (bind (_returnvalue_roll_3 _returnvalue_pitch_3 _returnvalue_yaw_3) (`KismetMathLibrary.BreakRotator` (`KismetMathLibrary.RLerp` (`KismetMathLibrary.MakeRotator` 0.0 0.0 _returnvalue_yaw) (`KismetMathLibrary.MakeRotator` 0.0 0.0 _returnvalue_yaw_2) _alpha true)))
          (`self.K2_SetActorRotation` (`KismetMathLibrary.MakeRotator` 0.0 0.0 _returnvalue_yaw_3)))
        (:`else`
          (goto _label_8 :!via `Stop`))))))

(event `EndAttackCombo`
  ;[0 0 0] Attack combo
  (set `self.AttackCounts` (- (`self.AttackCounts`) 1))
  (`self.RotateToPlayer`))

(event `Hit Handle`
  ;[0 0 0] Hit Reaction
  (bind _output_get (set `self.CurHP` (- (`self.CurHP`) 0.01)))
  (if (< _output_get 0.0)
    (if (not (`self.Dead`))
      (`self.Death`))))

(event `FireBall`
  (bind _spawnedfireball (`self.SpawnedFireBall`))
  (bind _returnvalue (`|SpawnActorFromClass` "/Game/Blueprints/BPA_FireBall.BPA_FireBall_C" (`KismetMathLibrary.MakeTransform` (`SceneComponent.GetSocketLocation` (`self.Mesh`) "Socket_SpreadFire")) "Undefined" "OverrideRootScale" null self null))
  (set `self.SpawnedFireBall` _returnvalue)
  (bind _target (`self.Target`)
    (:`then`
      (set `self.PlayerLocationWhenFireBallSpawned` (`self.K2_GetActorLocation` _target))
      (bind (_direction _alpha) (`Timeline|FireBallTime` :!via `PlayFromStart` :!label _label_9)
        (:`Update`
          (`/Engine/EditorBlueprintResources/StandardMacros.IsValid` _spawnedfireball
            (:`Is Valid`
              (`self.K2_SetActorLocation` _spawnedfireball (`KismetMathLibrary.VLerp` (`SceneComponent.GetSocketLocation` (`self.Mesh`) "Socket_SpreadFire") (`self.PlayerLocationWhenFireBallSpawned`) _alpha) false false))
            (:`Is Not Valid`
              (goto _label_9 :!via `Stop`))))
        (:`Finished`
          (bind _spawnedfireball_2 (`self.SpawnedFireBall`)
            (:`then`
              (`/Game/Blueprints/BPA_FireBall.EndOfFireBall` _spawnedfireball_2))
            (:`else`)))))
    (:`else`)))

(event `Stun`
  ;[0 0 0] Hit Reaction
  (set `self.EnableTick` false) ; Do not rotate actively to player during stun
  (set `self.AllowBehave?` false) ; Disable movement logic temporily
  (`self.PlayAnimMontage` null)
  (`|ExecutionSequence`
    (:`then_0`
      (bind (_direction _alpha) (`Timeline|KnockBack` :!via `PlayFromStart`) ; KnockBack time 0.5s
        (:`Update`
          (bind _target (`self.Target`)
            (:`then`
              (`self.K2_SetActorLocation` (`KismetMathLibrary.VLerp` (`self.K2_GetActorLocation`) (+ (`self.K2_GetActorLocation`) (* (`self.GetActorForwardVector` _target) (`self.KnockBackDistance`))) _alpha)))
            (:`else`)))))
    (:`then_1`
      (`KismetSystemLibrary.Delay` 2.0) ; Stun duration
      (if (not (`self.Dead`))
        (`AnimInstance.Montage_Stop` (`self.CastAnimIns`) 0.0 null)
        (set `self.AllowBehave?` true)
        (set `self.EnableTick` true)
        (`self.NextAttack`)))))

(event `Death`
  ;[0 0 0] Death
  (set `self.Dead` true)
  (set `self.AllowBehave?` false)
  (`KismetSystemLibrary.PrintString` "Dead!!")
  (`KismetSystemLibrary.K2_ClearAndInvalidateTimerHandle` (`self.CombatStartHandle`))
  (`AnimInstance.Montage_Stop` (`self.CastAnimIns`) 0.0 null)
  (if (`self.Fly?`)
    (`CharacterMovementComponent.SetMovementMode` (`self.CharacterMovement`) "MOVE_Falling" 0)
    (`KismetSystemLibrary.K2_SetTimer` null "CheckGround" 0.016 true)
    (bind _returnvalue (`self.PlayAnimMontage` "/Game/QuadrapedCreatures/MountainDragon/Animations/ANIM_MOUNTAIN_DRAGON_falling_Montage.ANIM_MOUNTAIN_DRAGON_falling_Montage" :!label _label_10))
    (`KismetSystemLibrary.Delay` _returnvalue)
    (if (`self.LoopFalling?`)
      (goto _label_10))
    (else
      (`self.PlayAnimMontage` "/Game/QuadrapedCreatures/MountainDragon/Animations/ANIM_MOUNTAIN_DRAGON_death_Montage.ANIM_MOUNTAIN_DRAGON_death_Montage")
      (`PrimitiveComponent.SetCollisionEnabled` (`self.CapsuleComponent`) "NoCollision")
      (`KismetSystemLibrary.Delay` 3.0)
      (`self.K2_DestroyActor`))))

(fn `INT_isAlive?`
  (returns (`Alive?` :type Boolean))
  (return false))

(fn `TurnInPlace`
  (params (R :type "Float (double-precision)"))
  (returns (RotationTime :type "Float (double-precision)") (NeedToRotate :type Boolean))
  (locals (L_RelativeRotation :type "Float (double-precision)") (L_RotationTime :type "Float (double-precision)" :default 0.0))
  (bind (_returnvalue_roll _returnvalue_pitch _returnvalue_yaw) (`KismetMathLibrary.BreakRotator` (`self.K2_GetActorRotation`)))
  (bind _l_relativerotation (`local.L_RelativeRotation`))
  (bind _l_relativerotation_2 (`local.L_RelativeRotation`))
  (bind _l_relativerotation_3 (`local.L_RelativeRotation`))
  (bind _target (`self.Target`)
    (:`then`
      (bind (_returnvalue_roll_2 _returnvalue_pitch_2 _returnvalue_yaw_2) (`KismetMathLibrary.BreakRotator` (`KismetMathLibrary.FindLookAtRotation` (`self.K2_GetActorLocation`) (`self.K2_GetActorLocation` _target))))
      (set `local.L_RelativeRotation` (- _returnvalue_yaw_2 _returnvalue_yaw))
      (if (or (and (> _l_relativerotation_2 0.0) (<= _l_relativerotation_2 90.0)) (and (> _l_relativerotation_2 -360.0) (<= _l_relativerotation_2 -270.0)))
        (bind _returnvalue (`self.PlayAnimMontage` "/Game/QuadrapedCreatures/MountainDragon/Animations/ANIM_MOUNTAIN_DRAGON_turn90Right_Montage.ANIM_MOUNTAIN_DRAGON_turn90Right_Montage"))
        (set `local.L_RotationTime` _returnvalue)
        (elif (or (and (> _l_relativerotation_3 90.0) (<= _l_relativerotation_3 180.0)) (and (> _l_relativerotation_3 -270.0) (<= _l_relativerotation_3 -180.0)))
          (bind _returnvalue_2 (`self.PlayAnimMontage` "/Game/QuadrapedCreatures/MountainDragon/Animations/ANIM_MOUNTAIN_DRAGON_turn90Right_Montage.ANIM_MOUNTAIN_DRAGON_turn90Right_Montage"))
          (set `local.L_RotationTime` _returnvalue_2)
          (elif (or (and (> _l_relativerotation 180.0) (<= _l_relativerotation 270.0)) (and (> _l_relativerotation -180.0) (<= _l_relativerotation -90.0)))
            (bind _returnvalue_3 (`self.PlayAnimMontage` "/Game/QuadrapedCreatures/MountainDragon/Animations/ANIM_MOUNTAIN_DRAGON_bite_Montage.ANIM_MOUNTAIN_DRAGON_bite_Montage"))
            (set `local.L_RotationTime` _returnvalue_3)
            (else
              (bind _returnvalue_4 (`self.PlayAnimMontage` "/Game/QuadrapedCreatures/MountainDragon/Animations/ANIM_MOUNTAIN_DRAGON_turn90Left_Montage.ANIM_MOUNTAIN_DRAGON_turn90Left_Montage"))
              (set `local.L_RotationTime` _returnvalue_4)))))
      (return (`local.L_RotationTime`) true))
    (:`else`)))

(fn `UserConstructionScript`
  (`SceneComponent.K2_SetRelativeLocation` (`self.Mesh`) (0.0 0.0 0.0) false false)
  (`SceneComponent.K2_AddRelativeLocation` (`self.Mesh`) (`KismetMathLibrary.MakeVector` 0.0 0.0 (- 0.0 (`CapsuleComponent.GetScaledCapsuleHalfHeight` (`self.CapsuleComponent`)))) false false)
  (`ActorComponent.SetAutoActivate` (`self.Mesh`) false))